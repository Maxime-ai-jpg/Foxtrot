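; BP_Door_out is an interactable door that opens once, when OpenDoor is called while the player is nearby.
; Box overlap begin and end events toggle PlayerIsClose, without checking which actor overlaps.
; OpenDoor checks that flag, then a DoOnce plays the OpenTime timeline, which lerps the Door component's relative location downward, with no closing logic.
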(event OnComponentBeginOverlap(Box)
  (params (OverlappedComponent :type Primitive%20Component%20Object%20Reference) (OtherActor :type Actor%20Object%20Reference) (OtherComp :type Primitive%20Component%20Object%20Reference) (OtherBodyIndex :type Integer) (bFromSweep :type Boolean) (SweepResult :type Hit%20Result%20Structure%20%28by%20ref%29))
  (Variables|Default|SetplayerIsClose? true))

(event OnComponentEndOverlap(Box)
  (params (OverlappedComponent :type Primitive%20Component%20Object%20Reference) (OtherActor :type Actor%20Object%20Reference) (OtherComp :type Primitive%20Component%20Object%20Reference) (OtherBodyIndex :type Integer))
  (Variables|Default|SetplayerIsClose? false))

(event Custom|Open%20Door
  (if (Variables|Default|GetplayerIsClose?)
    (Utilities|FlowControl|DoOnce false
      (:Completed
        (bind _newtrack_0 (Timeline|open%20time Play)
          (:Update
            (Transformation|SetRelativeLocation (Variables|Default|GetDoor) (Math|Vector|Lerp(Vector) "0.000000,-300.000000,0.000000" "0.000000,-300.000000,-850.000000" _newtrack_0) false false)))))))

(fn ConstructionScript)