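; BP_Door_Room_1 is a child door Blueprint for the first room that slides down when opened.
; An OpenDoor event runs once, playing a Timeline whose track drives the parent's MoveDoorDown function.
; A CodeIsGood flag is reset on BeginPlay, but its branch is unconnected, so opening relies on another object calling OpenDoor.
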(event EventOpenDoor
  ;[1 1 1] Avec ca ou alors sans branch et appler l'event dans le code du truc ou on met les symbols
  (Utilities|FlowControl|DoOnce false
    (:Completed
      (bind _newtrack_0 (Timeline|Timeline Play)
        (:Update
          (CallFunction|MoveDoorDown _newtrack_0))))))

(event EventBeginPlay
  (Variables|Default|SetCode%20is%20good%20? false))

(fn ConstructionScript
  (|CallParentFunction))

(fn MoveDoorDown
  (params (Alpha :type Float%20%28single-precision%29))
  (|CallParentFunction Alpha))