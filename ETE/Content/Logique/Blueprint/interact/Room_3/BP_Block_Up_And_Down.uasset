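; Room 3 block that continuously moves its Cube up and down along Z, starting at BeginPlay.
; MoveUp plays the UpTime timeline to lerp the relative location upward, and a second timeline lerps it back down through matching Move helpers.
; Both timelines chain from their Update pins through Delays, rather than from Finished, with the second re-calling MoveUp to repeat the cycle.
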(event Custom|Move%20Up
  (bind _1 (Timeline|up%20time PlayFromStart)
    (:Update
      (CallFunction|Move+ _1 "0, 0, 0" "0.000000,0.000000,200.000000")
      (Utilities|FlowControl|Delay 1.5)
      (bind _1_2 (Timeline|Timeline PlayFromStart)
        (:Update
          (CallFunction|Move- _1_2 "0.000000,0.000000,200.000000" "0, 0, 0")
          (Utilities|FlowControl|Delay 1.5)
          (CallFunction|MoveUp))))))

(event EventBeginPlay
  (CallFunction|MoveUp))

(fn ConstructionScript)

(fn Move+
  (params (Alpha :type Float%20%28single-precision%29) (A :type Vector) (B :type Vector))
  (Transformation|SetRelativeLocation (Variables|Default|GetCube) (Math|Vector|Lerp(Vector) A B Alpha) false false))

(fn Move-
  (params (Alpha :type Float%20%28single-precision%29) (A :type Vector) (B :type Vector))
  (Transformation|SetRelativeLocation (Variables|Default|GetCube) (Math|Vector|Lerp(Vector) A B Alpha) false false))