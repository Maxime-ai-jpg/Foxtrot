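; Child variant of a forward-and-backward block in Room 3 that moves back and forth along a diagonal path, forward and up, then back.
; MoveForward plays two timelines that feed Move with an alpha between fixed endpoints, and re-calls itself to loop.
; Each 1.5-second Delay hangs off timeline Update, so it counts from the leg's first update rather than its end.
; The Move overrides just call the parent.
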(event EventBeginPlay
  (|CallParentFunction) ; This node is disabled and will not be called.\nDrag off pins to build functionality.
)

(event EventMoveForward
  (bind _newtrack_0 (Timeline|Timeline_1 PlayFromStart)
    (:Update
      (CallFunction|Move+ _newtrack_0 "0, 0, 0" "250.000000,0.000000,200.000000")
      (Utilities|FlowControl|Delay 1.5)
      (bind _newtrack_0_2 (Timeline|Timeline_2 PlayFromStart)
        (:Update
          (CallFunction|Move- _newtrack_0_2 "250.000000,0.000000,200.000000" "0, 0, 0")
          (Utilities|FlowControl|Delay 1.5)
          (CallFunction|MoveForward))))))

(fn ConstructionScript
  (|CallParentFunction))

(fn Move+
  (params (Alpha :type Float%20%28single-precision%29) (A :type Vector :default "0, 0, 0") (B :type Vector :default "0, 0, 0"))
  (|CallParentFunction Alpha A B))

(fn Move-
  (params (Alpha :type Float%20%28single-precision%29) (A :type Vector :default "0, 0, 0") (B :type Vector :default "0, 0, 0"))
  (|CallParentFunction Alpha A B))