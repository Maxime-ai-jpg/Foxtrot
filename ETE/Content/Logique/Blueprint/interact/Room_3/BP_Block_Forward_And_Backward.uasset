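; Room 3 moving block that shuttles its Cube back and forth along local X in an endless loop, started on BeginPlay.
; Two timelines drive the forward and backward moves by lerping the Cube's relative location without sweep.
; Each timeline's Update output, rather than Finished, feeds a delay that triggers the opposite move, with the backward one calling MoveForward again.
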(event Custom|Move%20Forward
  (bind _1 (Timeline|Timeline PlayFromStart)
    (:Update
      (CallFunction|Move+ _1 "0, 0, 0" "200.000000,0.000000,0.000000")
      (Utilities|FlowControl|Delay 1.5)
      (bind _1_2 (Timeline|Timeline_0 PlayFromStart)
        (:Update
          (CallFunction|Move- _1_2 "200.000000,0.000000,0.000000" "0, 0, 0")
          (Utilities|FlowControl|Delay 1.5)
          (CallFunction|MoveForward))))))

(event EventBeginPlay
  (CallFunction|MoveForward))

(fn ConstructionScript)

(fn Move+
  (params (Alpha :type Float%20%28single-precision%29) (A :type Vector) (B :type Vector))
  (Transformation|SetRelativeLocation (Variables|Default|GetCube) (Math|Vector|Lerp(Vector) A B Alpha) false false))

(fn Move-
  (params (Alpha :type Float%20%28single-precision%29) (A :type Vector) (B :type Vector))
  (Transformation|SetRelativeLocation (Variables|Default|GetCube) (Math|Vector|Lerp(Vector) A B Alpha) false false))